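; BP_FlowTest is a test actor that automatically plays through a scripted NPC dialogue sequence.
; On BeginPlay it waits briefly, optionally resets the dialogue manager's flags, prints the player's tags, then starts a looping timer.
; Whenever no dialogue is active, each tick of that timer advances a counter: it triggers FemmeArme, Mechano, then FemmeArme again, and finally toggles the quest log.
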(event Custom|Retry
  (bind _returnvalue (Actor|GetActorOfClass "/Game/Blueprints/ClementTest/BP_Interact1ClementTestFemmeArme.BP_Interact1ClementTestFemmeArme_C"))
  (bind _returnvalue_2 (Actor|GetActorOfClass "/Game/Blueprints/ClementTest/BP_Interact1ClementTestMechano.BP_Interact1ClementTestMechano_C"))
  (bind _returnvalue_3 (Actor|GetActorOfClass "/Game/Blueprints/ClementTest/Dialogue/BP_DialogueManager.BP_DialogueManager_C"))
  (if (not (Variables|/Game/Blueprints/ClementTest/Dialogue/BP_DialogueManager.BP_DialogueManager_C|GetbIsActive _returnvalue_3))
    (Variables|Default|SetCounter (+ (Variables|Default|GetCounter) (Class|KismetSystemLibrary|MakeLiteralInteger 1)))
    (if (== (Variables|Default|GetCounter) (Class|KismetSystemLibrary|MakeLiteralInteger 2))
      (Default|Interact (Variables|/Game/Blueprints/ClementTest/BP_Interact1ClementTestMechano.BP_Interact1ClementTestMechano_C|GetDialogueNPC _returnvalue_2))
      (elif (or (== (Variables|Default|GetCounter) (Class|KismetSystemLibrary|MakeLiteralInteger 1)) (== (Variables|Default|GetCounter) (Class|KismetSystemLibrary|MakeLiteralInteger 3)))
        (Default|Interact (Variables|/Game/Blueprints/ClementTest/BP_Interact1ClementTestFemmeArme.BP_Interact1ClementTestFemmeArme_C|GetDialogueNPC _returnvalue))
        (elif (== (Variables|Default|GetCounter) (Class|KismetSystemLibrary|MakeLiteralInteger 4))
          (Default|ToggleQuestLog _returnvalue_3))))))

(event EventBeginPlay
  (Utilities|FlowControl|Delay 1.0)
  (bind _returnvalue (Actor|GetActorOfClass "/Game/Blueprints/ClementTest/Dialogue/BP_DialogueManager.BP_DialogueManager_C"))
  (if (Variables|Default|GetbResetAtStart)
    (Default|ResetFlags _returnvalue))
  (Development|PrintString (Utilities|String|Append "[FlowTest] tags au demarrage : " (GameplayTags|GetDebugStringfromGameplayTagContainer (Variables|/Game/Blueprints/ClementTest/Dialogue/BP_DialogueManager.BP_DialogueManager_C|GetPlayerFlags _returnvalue))) false)
  (Utilities|Time|SetTimerbyFunctionName self "Retry" 3.0 true))

(event Collision|EventActorBeginOverlap
  (params (OtherActor :type Actor%20Object%20Reference)))

(event EventTick
  (params (DeltaSeconds :type Float%20%28single-precision%29)))

(fn ConstructionScript)