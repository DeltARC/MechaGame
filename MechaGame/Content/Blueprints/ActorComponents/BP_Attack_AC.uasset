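; BP_Attack_AC is an actor component that gives its owner a short-range forward attack.
; Its Attack event sphere-traces ahead from the owner's location along its forward vector, ignoring the owner, against world, pawn and destructible objects.
; A hit actor with a BP_Health_AC component receives fixed damage through that component's TakeDamage, so any actor with health can be hit.
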(event Custom|Attack
  (bind _returnvalue (Components|GetOwner))
  (bind _returnvalue_2 (Transformation|GetActorLocation _returnvalue))
  (bind (_outhit _returnvalue_3) (Collision|SphereTraceForObjects _returnvalue_2 (+ _returnvalue_2 (* (Transformation|GetActorForwardVector _returnvalue) 3e+02)) 0.0 (Utilities|Array|MakeArray "ObjectTypeQuery1" "ObjectTypeQuery3" "ObjectTypeQuery2" "ObjectTypeQuery6") false (Utilities|Array|MakeArray (Components|GetOwner)) "None"))
  (if _returnvalue_3
    (Utilities|IsValid (Actor|GetComponentbyClass (.HitActor (Collision|BreakHitResult _outhit)) "/Game/Blueprints/ActorComponents/BP_Health_AC.BP_Health_AC_C")
      (:Is%20Valid
        (Default|TakeDamage (Actor|GetComponentbyClass (.HitActor (Collision|BreakHitResult _outhit)) "/Game/Blueprints/ActorComponents/BP_Health_AC.BP_Health_AC_C") 2e+01)))))