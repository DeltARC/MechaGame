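; Actor component that makes its owner a talkable NPC, starting dialogue from its DialogueTable through a shared BP_DialogueManager it finds or spawns.
; On BeginPlay it validates the table against every possible start node.
; Interact picks the start node from the first entry tag matching the manager's player flags, falling back to a default.
; It can blend the camera to the owner, restoring the previous view when its own dialogue ends.
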(event Custom|Interact
  (bind _returnvalue (Game|GetPlayerController 0))
  (bind _dialoguemanager (CallFunction|GetManager))
  (bind _nodeid (CallFunction|ResolveStartNodeID))
  (if (and (not (Variables|/Game/Blueprints/ClementTest/Dialogue/BP_DialogueManager.BP_DialogueManager_C|GetbIsActive _dialoguemanager)) (not (Variables|Default|GetbOwnsCurrentDialogue)))
    (Variables|Default|SetbOwnsCurrentDialogue true)
    (Variables|Default|SetPreviousViewTarget (Pawn|GetViewTarget _returnvalue))
    (if (Variables|Dialogue|GetbFocusCameraOnOwner)
      (Game|Player|SetViewTargetwithBlend _returnvalue (Components|GetOwner) (Variables|Dialogue|GetCameraBlendTime) "VTBlend_Linear" 0.0 false)
      (Utilities|FlowControl|Delay (Variables|Dialogue|GetCameraBlendTime))
      (Default|StartDialogue _dialoguemanager (Variables|Dialogue|GetDialogueTable) _nodeid (Variables|Dialogue|GetWidgetName))
      (else
        (Default|StartDialogue _dialoguemanager (Variables|Dialogue|GetDialogueTable) _nodeid (Variables|Dialogue|GetWidgetName))))))

(event Custom|HandleDialogueEnded
  (if (Variables|Default|GetbOwnsCurrentDialogue)
    (Variables|Default|SetbOwnsCurrentDialogue false)
    (if (Variables|Dialogue|GetbFocusCameraOnOwner)
      (Game|Player|SetViewTargetwithBlend (Game|GetPlayerController 0) (Variables|Default|GetPreviousViewTarget) (Variables|Dialogue|GetCameraBlendTime) "VTBlend_Linear" 0.0 false))))

(event EventBeginPlay
  (bind _dialoguemanager (CallFunction|GetManager))
  (bind _nodeids (CallFunction|GetAllStartNodeIDs))
  (EventDispatchers|BindEventtoOnDialogueEnded _dialoguemanager (EventDispatchers|CreateEvent :!event Custom|HandleDialogueEnded))
  (Utilities|IsValid (Variables|Dialogue|GetDialogueTable)
    (:Is%20Valid
      (Default|ValidateTable _dialoguemanager (Variables|Dialogue|GetDialogueTable) _nodeids))
    (:Is%20Not%20Valid
      (Development|PrintString (Utilities|String|Append "[Dialogue] ATTENTION : aucune DialogueTable sur le composant de dialogue de " (Utilities|GetDisplayName (Components|GetOwner))) true true "(R=1.0,G=0.8,B=0.1,A=1.0)" 15.0))))

(event EventTick
  (params (DeltaSeconds :type Float%20%28single-precision%29)))

(fn GetManager
  (Utilities|IsValid (Variables|Default|GetManager)
    (:Is%20Valid
      (return (Variables|Default|GetManager)))
    (:Is%20Not%20Valid
      (bind _returnvalue (Actor|GetActorOfClass "/Game/Blueprints/ClementTest/Dialogue/BP_DialogueManager.BP_DialogueManager_C"))
      (Utilities|IsValid _returnvalue
        (:Is%20Valid
          (Variables|Default|SetManager _returnvalue)
          (return (Variables|Default|GetManager)))
        (:Is%20Not%20Valid
          (bind _returnvalue_2 (Game|SpawnActorfromClass "/Game/Blueprints/ClementTest/Dialogue/BP_DialogueManager.BP_DialogueManager_C" (Math|Transform|MakeTransform "0, 0, 0") "AlwaysSpawn" "MultiplyWithRoot" 0 0))
          (Variables|Default|SetManager _returnvalue_2)
          (return (Variables|Default|GetManager)))))))

(fn ResolveStartNodeID
  (bind _dialoguemanager (CallFunction|GetManager))
  (for _index (range 0 (- (Utilities|Array|Length (Variables|Dialogue|GetEntryPointTags)) (Class|KismetSystemLibrary|MakeLiteralInteger 1)))
    (if (and (Utilities|Array|IsValidIndex (Variables|Dialogue|GetEntryPointNodeIDs) _index) (GameplayTags|HasTag (Variables|/Game/Blueprints/ClementTest/Dialogue/BP_DialogueManager.BP_DialogueManager_C|GetPlayerFlags _dialoguemanager) (Utilities|Array|Get(acopy) (Variables|Dialogue|GetEntryPointTags) _index) true))
      (return (Utilities|Array|Get(acopy) (Variables|Dialogue|GetEntryPointNodeIDs) _index))))
  (return (Variables|Dialogue|GetStartNodeID)))

(fn GetAllStartNodeIDs
  (Utilities|Array|Clear (LocalVariables|GetIDs))
  (Utilities|Array|Add (LocalVariables|GetIDs) (Variables|Dialogue|GetStartNodeID))
  (Utilities|Array|AppendArray (LocalVariables|GetIDs) (Variables|Dialogue|GetEntryPointNodeIDs))
  (return (LocalVariables|GetIDs)))