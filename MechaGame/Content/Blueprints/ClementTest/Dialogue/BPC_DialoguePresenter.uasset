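; BPC_DialoguePresenter is the dialogue UI component of BP_DialogueManager, driven by its started, node-changed and ended events.
; It creates a Mechano or FemmeArme widget by name and switches player input to the UI until dialogue ends.
; Each line types out on a looping timer with a skip button, then shows choices with persuasion/intimidation prefixes or Continue.
; All choice buttons share one handler, resolving the clicked index by keyboard focus or hover.
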(event Custom|HandleDialogueStarted
  (bind _returnvalue (Game|GetPlayerController 0))
  (CallFunction|CreateDialogueWidget (Variables|/Game/Blueprints/ClementTest/Dialogue/BP_DialogueManager.BP_DialogueManager_C|GetCurrentWidgetName (Variables|Default|GetManager)))
  (UserInterface|Viewport|AddtoViewport (Variables|Default|GetWidget) 0)
  (for _array_element (Variables|Default|GetChoiceButtons)
    (EventDispatchers|BindEventtoOnClicked _array_element (EventDispatchers|CreateEvent :!event Custom|HandleChoiceClicked)))
  (EventDispatchers|BindEventtoOnClicked (Variables|Default|GetLeaveButton) (EventDispatchers|CreateEvent :!event Custom|HandleLeaveClicked))
  (Variables|Default|SetbPreviousShowCursor (Variables|/Script/Engine.PlayerController|GetbShowMouseCursor _returnvalue))
  (Variables|/Script/Engine.PlayerController|SetbShowMouseCursor _returnvalue true)
  (Input|SetInputModeGameandUI _returnvalue 0 "DoNotLock" true false)
  (Input|SetIgnoreMoveInput _returnvalue true)
  (Input|SetIgnoreLookInput _returnvalue true))

(event Custom|HandleNodeChanged
  (CallFunction|ShowLine))

(event Custom|TypeTick
  (Variables|Default|SetVisibleChars (+ (Variables|Default|GetVisibleChars) (Class|KismetSystemLibrary|MakeLiteralInteger 1)))
  (Rendering|Components|TextRender|SetText (Variables|Default|GetLineText) (Utilities|Text|ToText(String) (Utilities|String|Left (Variables|Default|GetFullLine) (Variables|Default|GetVisibleChars))))
  (if (>= (Variables|Default|GetVisibleChars) (Utilities|String|Len (Variables|Default|GetFullLine)))
    (CallFunction|FinishTyping)))

(event Custom|HandleChoiceClicked
  (if (Variables|Default|GetbIsTyping)
    (CallFunction|FinishTyping)
    (else
      (bind _index (CallFunction|GetClickedIndex))
      (bind _choices (Default|GetAvailableChoices (Variables|Default|GetManager)))
      (if (Utilities|Array|IsEmpty _choices)
        (Default|Continue (Variables|Default|GetManager))
        (elif (>= _index (Class|KismetSystemLibrary|MakeLiteralInteger))
          (Default|SelectChoice (Variables|Default|GetManager) _index))))))

(event Custom|HandleLeaveClicked
  (Default|EndDialogue (Variables|Default|GetManager)))

(event Custom|HandleDialogueEnded
  (bind _returnvalue (Game|GetPlayerController 0))
  (Variables|Default|SetbIsTyping false)
  (Utilities|Time|ClearandInvalidateTimerbyHandle (Variables|Default|GetTypeTimer))
  (Widget|RemovefromParent (Variables|Default|GetWidget))
  (Variables|/Script/Engine.PlayerController|SetbShowMouseCursor _returnvalue (Variables|Default|GetbPreviousShowCursor))
  (Input|SetInputModeGameOnly _returnvalue false)
  (Input|SetIgnoreMoveInput _returnvalue false)
  (Input|SetIgnoreLookInput _returnvalue false))

(event EventBeginPlay
  (bind _asbp_dialogue_manager (Utilities|Casting|CastToBP_DialogueManager (Components|GetOwner))
    (:then
      (Variables|Default|SetManager _asbp_dialogue_manager)
      (EventDispatchers|BindEventtoOnDialogueStarted _asbp_dialogue_manager (EventDispatchers|CreateEvent :!event Custom|HandleDialogueStarted))
      (EventDispatchers|BindEventtoOnNodeChanged _asbp_dialogue_manager (EventDispatchers|CreateEvent :!event Custom|HandleNodeChanged))
      (EventDispatchers|BindEventtoOnDialogueEnded _asbp_dialogue_manager (EventDispatchers|CreateEvent :!event Custom|HandleDialogueEnded)))
    (:CastFailed
      (Development|PrintString "[Dialogue] ERREUR : BPC_DialoguePresenter doit etre un composant de BP_DialogueManager." true true "(R=1.0,G=0.2,B=0.2,A=1.0)" 15.0))))

(event EventTick
  (params (DeltaSeconds :type Float%20%28single-precision%29)))

(fn CreateDialogueWidget
  (params (WidgetName :type Name))
  (Utilities|Array|Clear (Variables|Default|GetChoiceButtons))
  (Utilities|Array|Clear (Variables|Default|GetChoiceTexts))
  (if (== WidgetName (Utilities|String|MakeLiteralString "Mechano"))
    (bind _returnvalue (UserInterface|CreateWidget "/Game/Widgets/ClementTest/DialogueChoix/WBP_DialogueChoixMechano.WBP_DialogueChoixMechano_C" (Game|GetPlayerController 0)))
    (Variables|Default|SetWidget _returnvalue)
    (Variables|Default|SetLineText (Variables|/Game/Widgets/ClementTest/DialogueChoix/WBP_DialogueChoixMechano.WBP_DialogueChoixMechano_C|GetTextPNJ _returnvalue))
    (Variables|Default|SetPortrait (Variables|/Game/Widgets/ClementTest/DialogueChoix/WBP_DialogueChoixMechano.WBP_DialogueChoixMechano_C|GetImage_283 _returnvalue))
    (Variables|Default|SetLeaveButton (Variables|/Game/Widgets/ClementTest/DialogueChoix/WBP_DialogueChoixMechano.WBP_DialogueChoixMechano_C|GetButtonLeave _returnvalue))
    (Utilities|Array|Add (Variables|Default|GetChoiceButtons) (Variables|/Game/Widgets/ClementTest/DialogueChoix/WBP_DialogueChoixMechano.WBP_DialogueChoixMechano_C|GetButtonChoix1 _returnvalue))
    (Utilities|Array|Add (Variables|Default|GetChoiceButtons) (Variables|/Game/Widgets/ClementTest/DialogueChoix/WBP_DialogueChoixMechano.WBP_DialogueChoixMechano_C|GetButtonChoix2 _returnvalue))
    (Utilities|Array|Add (Variables|Default|GetChoiceTexts) (Variables|/Game/Widgets/ClementTest/DialogueChoix/WBP_DialogueChoixMechano.WBP_DialogueChoixMechano_C|GetChoix1 _returnvalue))
    (Utilities|Array|Add (Variables|Default|GetChoiceTexts) (Variables|/Game/Widgets/ClementTest/DialogueChoix/WBP_DialogueChoixMechano.WBP_DialogueChoixMechano_C|GetChoix2 _returnvalue))
    (else
      (bind _returnvalue_2 (UserInterface|CreateWidget "/Game/Widgets/ClementTest/DialogueChoix/WBP_DialogueChoixFemmeArme.WBP_DialogueChoixFemmeArme_C" (Game|GetPlayerController 0)))
      (Variables|Default|SetWidget _returnvalue_2)
      (Variables|Default|SetLineText (Variables|/Game/Widgets/ClementTest/DialogueChoix/WBP_DialogueChoixFemmeArme.WBP_DialogueChoixFemmeArme_C|GetTextPNJ _returnvalue_2))
      (Variables|Default|SetPortrait (Variables|/Game/Widgets/ClementTest/DialogueChoix/WBP_DialogueChoixFemmeArme.WBP_DialogueChoixFemmeArme_C|GetImage_283 _returnvalue_2))
      (Variables|Default|SetLeaveButton (Variables|/Game/Widgets/ClementTest/DialogueChoix/WBP_DialogueChoixFemmeArme.WBP_DialogueChoixFemmeArme_C|GetButtonLeave _returnvalue_2))
      (Utilities|Array|Add (Variables|Default|GetChoiceButtons) (Variables|/Game/Widgets/ClementTest/DialogueChoix/WBP_DialogueChoixFemmeArme.WBP_DialogueChoixFemmeArme_C|GetButtonChoix1 _returnvalue_2))
      (Utilities|Array|Add (Variables|Default|GetChoiceButtons) (Variables|/Game/Widgets/ClementTest/DialogueChoix/WBP_DialogueChoixFemmeArme.WBP_DialogueChoixFemmeArme_C|GetButtonChoix2 _returnvalue_2))
      (Utilities|Array|Add (Variables|Default|GetChoiceTexts) (Variables|/Game/Widgets/ClementTest/DialogueChoix/WBP_DialogueChoixFemmeArme.WBP_DialogueChoixFemmeArme_C|GetChoix1 _returnvalue_2))
      (Utilities|Array|Add (Variables|Default|GetChoiceTexts) (Variables|/Game/Widgets/ClementTest/DialogueChoix/WBP_DialogueChoixFemmeArme.WBP_DialogueChoixFemmeArme_C|GetChoix2 _returnvalue_2)))))

(fn UpdateSpeaker
  (bind _manager (Variables|Default|GetManager))
  (bind _currentnode (Variables|/Game/Blueprints/ClementTest/Dialogue/BP_DialogueManager.BP_DialogueManager_C|GetCurrentNode _manager))
  (bind (_speaker _mood) (Utilities|Struct|BreakS_DialogueNode _currentnode))
  (bind _portraits (Variables|/Game/Blueprints/ClementTest/Dialogue/BP_DialogueSpeakerData.BP_DialogueSpeakerData_C|GetPortraits _speaker))
  (bind (_value _returnvalue) (Utilities|Map|Find _portraits _mood))
  (Utilities|IsValid _speaker
    (:Is%20Valid
      (if _returnvalue
        (Variables|/Script/UMG.Image|SetBrush (Variables|Default|GetPortrait) (Class|WidgetBlueprintLibrary|MakeBrushfromTexture _value)))
      (Utilities|IsValid (Variables|Default|GetNameText)
        (:Is%20Valid
          (Rendering|Components|TextRender|SetText (Variables|Default|GetNameText) (Variables|/Game/Blueprints/ClementTest/Dialogue/BP_DialogueSpeakerData.BP_DialogueSpeakerData_C|GetDisplayName _speaker)))))))

(fn ShowLine
  (CallFunction|UpdateSpeaker)
  (Variables|Default|SetFullLine (Utilities|String|ToString(Text) (.Line (Utilities|Struct|BreakS_DialogueNode (Variables|/Game/Blueprints/ClementTest/Dialogue/BP_DialogueManager.BP_DialogueManager_C|GetCurrentNode (Variables|Default|GetManager))))))
  (Variables|Default|SetVisibleChars 0)
  (Variables|Default|SetbIsTyping true)
  (Rendering|Components|TextRender|SetText (Variables|Default|GetLineText) (Class|KismetTextLibrary|GetEmptyText))
  (CallFunction|ShowSkipButton)
  (Utilities|Time|ClearandInvalidateTimerbyHandle (Variables|Default|GetTypeTimer))
  (bind _returnvalue (Utilities|Time|SetTimerbyFunctionName self "TypeTick" (Variables|Dialogue|Reglages|GetTypewriterInterval) true))
  (Variables|Default|SetTypeTimer _returnvalue))

(fn ShowSkipButton
  (for _index (range 0 (- (Utilities|Array|Length (Variables|Default|GetChoiceButtons)) (Class|KismetSystemLibrary|MakeLiteralInteger 1)))
    (if (== _index (Class|KismetSystemLibrary|MakeLiteralInteger))
      (Widget|SetVisibility (Utilities|Array|Get(acopy) (Variables|Default|GetChoiceButtons) _index) "Visible")
      (else
        (Widget|SetVisibility (Utilities|Array|Get(acopy) (Variables|Default|GetChoiceButtons) _index) "Hidden"))))
  (if (Utilities|Array|IsNotEmpty (Variables|Default|GetChoiceTexts))
    (Rendering|Components|TextRender|SetText (Utilities|Array|Get(acopy) (Variables|Default|GetChoiceTexts)) (Variables|Dialogue|Reglages|GetSkipLabel)))
  (if (Utilities|Array|IsNotEmpty (Variables|Default|GetChoiceButtons))
    (Widget|SetKeyboardFocus (Utilities|Array|Get(acopy) (Variables|Default|GetChoiceButtons)))))

(fn ShowChoices
  (bind _choices (Default|GetAvailableChoices (Variables|Default|GetManager)))
  (for _index (range 0 (- (Utilities|Array|Length (Variables|Default|GetChoiceButtons)) (Class|KismetSystemLibrary|MakeLiteralInteger 1)))
    (if (< _index (Utilities|Array|Length _choices))
      (bind _label (CallFunction|GetChoiceLabel (Utilities|Array|Get(acopy) _choices _index)))
      (Rendering|Components|TextRender|SetText (Utilities|Array|Get(acopy) (Variables|Default|GetChoiceTexts) _index) _label)
      (Widget|SetVisibility (Utilities|Array|Get(acopy) (Variables|Default|GetChoiceButtons) _index) "Visible")
      (elif (and (== (Utilities|Array|Length _choices) (Class|KismetSystemLibrary|MakeLiteralInteger)) (== _index (Class|KismetSystemLibrary|MakeLiteralInteger)))
        (Rendering|Components|TextRender|SetText (Utilities|Array|Get(acopy) (Variables|Default|GetChoiceTexts) _index) (Variables|Dialogue|Reglages|GetContinueLabel))
        (Widget|SetVisibility (Utilities|Array|Get(acopy) (Variables|Default|GetChoiceButtons) _index) "Visible")
        (else
          (Widget|SetVisibility (Utilities|Array|Get(acopy) (Variables|Default|GetChoiceButtons) _index) "Hidden")))))
  (if (> (Utilities|Array|Length _choices) (Utilities|Array|Length (Variables|Default|GetChoiceButtons)))
    (Development|PrintString "[Dialogue] ATTENTION : ce noeud propose plus de choix que le widget n'a de boutons, les derniers ne sont pas affiches." true true "(R=1.0,G=0.8,B=0.1,A=1.0)" 1e+01))
  (if (Utilities|Array|IsNotEmpty (Variables|Default|GetChoiceButtons))
    (Widget|SetKeyboardFocus (Utilities|Array|Get(acopy) (Variables|Default|GetChoiceButtons)))))

(fn FinishTyping
  (if (Variables|Default|GetbIsTyping)
    (Variables|Default|SetbIsTyping false)
    (Utilities|Time|ClearandInvalidateTimerbyHandle (Variables|Default|GetTypeTimer))
    (Rendering|Components|TextRender|SetText (Variables|Default|GetLineText) (Utilities|Text|ToText(String) (Variables|Default|GetFullLine)))
    (CallFunction|ShowChoices)))

(fn GetClickedIndex
  (for _index (range 0 (- (Utilities|Array|Length (Variables|Default|GetChoiceButtons)) (Class|KismetSystemLibrary|MakeLiteralInteger 1)))
    (if (Class|Widget|HasKeyboardFocus (Utilities|Array|Get(acopy) (Variables|Default|GetChoiceButtons) _index))
      (return _index)))
  (for _index_2 (range 0 (- (Utilities|Array|Length (Variables|Default|GetChoiceButtons)) (Class|KismetSystemLibrary|MakeLiteralInteger 1)))
    (if (Widget|IsHovered (Utilities|Array|Get(acopy) (Variables|Default|GetChoiceButtons) _index_2))
      (return _index_2)))
  (return -1))

(fn GetChoiceLabel
  (params (Choice :type S%20Dialogue%20Choice%20Structure))
  (bind (_text _nextnodeid _condition _tagstogrant _tagstoremove _choicetype) (Utilities|Struct|BreakS_DialogueChoice Choice))
  (if (Utilities|Enum|Equal(Enum) _choicetype (Utilities|Enum|LiteralenumE_ChoiceType "NewEnumerator1"))
    (return (Utilities|Text|ToText(String) (Utilities|String|Append (Utilities|String|ToString(Text) (Variables|Dialogue|Reglages|GetPersuasionPrefix)) (Utilities|String|ToString(Text) _text))))
    (elif (Utilities|Enum|Equal(Enum) _choicetype (Utilities|Enum|LiteralenumE_ChoiceType "NewEnumerator2"))
      (return (Utilities|Text|ToText(String) (Utilities|String|Append (Utilities|String|ToString(Text) (Variables|Dialogue|Reglages|GetIntimidationPrefix)) (Utilities|String|ToString(Text) _text))))
      (else
        (return _text)))))