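; Dialogue manager actor that runs branching conversations from DataTables and holds the player's gameplay-tag flags.
; Each node filters its choices by tag query; picking one edits the flags, fires dispatchers and moves to the next node.
; Flag changes optionally persist through BP_DialogueSave, with hotkeys for flag reset and quest log toggle.
; ValidateTable traverses the node graph to report broken links, unreachable nodes and potential choiceless dead ends.
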(event Custom|ToggleQuestLog
  (Default|Toggle (Variables|Default|GetQuestLog)))

(event Custom|ResetSavedFlags
  (CallFunction|ResetFlags))

(event EventBeginPlay
  (Input|EnableInput (Game|GetPlayerController 0))
  (CallFunction|LoadFlags))

(event Collision|EventActorBeginOverlap
  (params (OtherActor :type Actor%20Object%20Reference)))

(event EventTick
  (params (DeltaSeconds :type Float%20%28single-precision%29)))

(event Input|KeyboardEvents|J
  (params (Key :type Key%20Structure))
  (:Pressed
    (Default|Toggle (Variables|Default|GetQuestLog))))

(event Input|KeyboardEvents|F6
  (params (Key :type Key%20Structure))
  (:Pressed
    (CallFunction|ResetFlags)))

(fn ConstructionScript)

(fn StartDialogue
  (params (Table :type Data%20Table%20Object%20Reference) (StartNodeID :type Name) (WidgetName :type Name))
  (if (Variables|Default|GetbIsActive)
    (Development|PrintString "[Dialogue] StartDialogue ignore : un dialogue est deja en cours." true true "(R=0.000000,G=0.660000,B=1.000000,A=1.000000)" 5.0)
    (else
      (Variables|Default|SetCurrentTable Table)
      (Variables|Default|SetCurrentWidgetName WidgetName)
      (Variables|Default|SetbIsActive true)
      (Default|CallOnDialogueStarted)
      (CallFunction|GotoNode StartNodeID))))

(fn GotoNode
  (params (NodeID :type Name))
  (if (== NodeID (Utilities|String|MakeLiteralString "None"))
    (CallFunction|EndDialogue)
    (else
      (bind _returnvalue (Utilities|GetDataTableRow (Variables|Default|GetCurrentTable) NodeID)
        (:then
          (Variables|Default|SetCurrentNodeID NodeID)
          (Variables|Default|SetCurrentNode _returnvalue)
          (CallFunction|RefreshAvailableChoices)
          (Default|CallOnNodeChanged))
        (:RowNotFound
          (Development|PrintString (Utilities|String|Append "[Dialogue] ERREUR : noeud introuvable dans la DataTable : " (Utilities|String|ToString(Name) NodeID)) true true "(R=1.0,G=0.2,B=0.2,A=1.0)" 1e+01)
          (CallFunction|EndDialogue))))))

(fn RefreshAvailableChoices
  (Utilities|Array|Clear (Variables|Default|GetAvailableChoices))
  (for _array_element (.Choices (Utilities|Struct|BreakS_DialogueNode (Variables|Default|GetCurrentNode)))
    (if (or (GameplayTags|IsTagQueryEmpty (.Condition (Utilities|Struct|BreakS_DialogueChoice _array_element))) (GameplayTags|DoesContainerMatchTagQuery (Variables|Default|GetPlayerFlags) (.Condition (Utilities|Struct|BreakS_DialogueChoice _array_element))))
      (Utilities|Array|Add (Variables|Default|GetAvailableChoices) _array_element))))

(fn SelectChoice
  (params (Index :type Integer))
  (if (and (Variables|Default|GetbIsActive) (Utilities|Array|IsValidIndex (Variables|Default|GetAvailableChoices) Index))
    (Variables|Default|SetLastChoice (Utilities|Array|Get(acopy) (Variables|Default|GetAvailableChoices) Index))
    (CallFunction|RemoveFlags (.TagsToRemove (Utilities|Struct|BreakS_DialogueChoice (Variables|Default|GetLastChoice))))
    (CallFunction|AddFlags (.TagsToGrant (Utilities|Struct|BreakS_DialogueChoice (Variables|Default|GetLastChoice))))
    (Default|CallOnChoiceSelected)
    (CallFunction|GotoNode (.NextNodeID (Utilities|Struct|BreakS_DialogueChoice (Variables|Default|GetLastChoice))))
    (else
      (Development|PrintString "[Dialogue] SelectChoice ignore : pas de dialogue en cours ou index de choix invalide." true true "(R=0.000000,G=0.660000,B=1.000000,A=1.000000)" 5.0))))

(fn Continue
  (if (Variables|Default|GetbIsActive)
    (CallFunction|GotoNode (.NextNodeID (Utilities|Struct|BreakS_DialogueNode (Variables|Default|GetCurrentNode))))))

(fn EndDialogue
  (if (Variables|Default|GetbIsActive)
    (Variables|Default|SetbIsActive false)
    (Variables|Default|SetCurrentNodeID "None")
    (Default|CallOnDialogueEnded)))

(fn GetAvailableChoices
  (return (Variables|Default|GetAvailableChoices)))

(fn AddFlags
  (params (Tags :type Gameplay%20Tag%20Container%20Structure))
  (GameplayTags|AppendGameplayTagContainers (Variables|Default|GetPlayerFlags) Tags)
  (Default|CallOnFlagsChanged)
  (CallFunction|SaveFlags))

(fn RemoveFlags
  (params (Tags :type Gameplay%20Tag%20Container%20Structure))
  (for _array_element (GameplayTags|BreakGameplayTagContainer Tags)
    (GameplayTags|RemoveGameplayTag (Variables|Default|GetPlayerFlags) _array_element :!class /Script/GameplayTags.BlueprintGameplayTagLibrary))
  (Default|CallOnFlagsChanged)
  (CallFunction|SaveFlags))

(fn AddFlag
  (params (Tag :type Gameplay%20Tag%20Structure))
  (GameplayTags|AddGameplayTag (Variables|Default|GetPlayerFlags) Tag :!class /Script/GameplayTags.BlueprintGameplayTagLibrary)
  (Default|CallOnFlagsChanged)
  (CallFunction|SaveFlags))

(fn RemoveFlag
  (params (Tag :type Gameplay%20Tag%20Structure))
  (GameplayTags|RemoveGameplayTag (Variables|Default|GetPlayerFlags) Tag :!class /Script/GameplayTags.BlueprintGameplayTagLibrary)
  (Default|CallOnFlagsChanged)
  (CallFunction|SaveFlags))

(fn HasFlag
  (params (Tag :type Gameplay%20Tag%20Structure))
  (return (GameplayTags|HasTag (Variables|Default|GetPlayerFlags) Tag true)))

(fn ValidateTable
  (params (Table :type Data%20Table%20Object%20Reference) (StartNodeIDs :type Array%20of%20Names))
  (Utilities|Array|Clear (LocalVariables|GetVisited))
  (Utilities|Array|Clear (LocalVariables|GetQueue))
  (Utilities|Array|AppendArray (LocalVariables|GetQueue) StartNodeIDs)
  (while (Utilities|Array|IsNotEmpty (LocalVariables|GetQueue))
    (LocalVariables|SetCheckID (Utilities|Array|Get(acopy) (LocalVariables|GetQueue) (Utilities|Array|LastIndex (LocalVariables|GetQueue))))
    (Utilities|Array|RemoveIndex (LocalVariables|GetQueue) (Utilities|Array|LastIndex (LocalVariables|GetQueue)))
    (if (and (!= (LocalVariables|GetCheckID) (Utilities|String|MakeLiteralString "None")) (not (Utilities|Array|ContainsItem (LocalVariables|GetVisited) (LocalVariables|GetCheckID))))
      (Utilities|Array|Add (LocalVariables|GetVisited) (LocalVariables|GetCheckID))
      (bind _returnvalue (Utilities|GetDataTableRow Table (LocalVariables|GetCheckID))
        (:then
          (LocalVariables|SetCheckNode _returnvalue)
          (Utilities|Array|Add (LocalVariables|GetQueue) (.NextNodeID (Utilities|Struct|BreakS_DialogueNode (LocalVariables|GetCheckNode))))
          (LocalVariables|SetFreeChoices 0)
          (for _array_element (.Choices (Utilities|Struct|BreakS_DialogueNode (LocalVariables|GetCheckNode)))
            (Utilities|Array|Add (LocalVariables|GetQueue) (.NextNodeID (Utilities|Struct|BreakS_DialogueChoice _array_element)))
            (if (GameplayTags|IsTagQueryEmpty (.Condition (Utilities|Struct|BreakS_DialogueChoice _array_element)))
              (LocalVariables|SetFreeChoices (+ (LocalVariables|GetFreeChoices) (Class|KismetSystemLibrary|MakeLiteralInteger 1)))))
          (if (and (Utilities|Array|IsNotEmpty (.Choices (Utilities|Struct|BreakS_DialogueNode (LocalVariables|GetCheckNode)))) (and (== (LocalVariables|GetFreeChoices) (Class|KismetSystemLibrary|MakeLiteralInteger)) (== (.NextNodeID (Utilities|Struct|BreakS_DialogueNode (LocalVariables|GetCheckNode))) (Utilities|String|MakeLiteralString "None"))))
            (Development|PrintString (Utilities|String|Append "[Dialogue] ATTENTION : tous les choix de ce noeud sont conditionnels et il n'a pas de NextNodeID, le dialogue peut s'y terminer sans choix : " (Utilities|String|ToString(Name) (LocalVariables|GetCheckID))) true true "(R=1.0,G=0.8,B=0.1,A=1.0)" 15.0)))
        (:RowNotFound
          (Development|PrintString (Utilities|String|Append "[Dialogue] ERREUR : un NextNodeID ou un point d'entree pointe vers un noeud inexistant : " (Utilities|String|ToString(Name) (LocalVariables|GetCheckID))) true true "(R=1.0,G=0.2,B=0.2,A=1.0)" 15.0)))))
  (bind _outrownames (DataTable|GetDataTableRowNames Table))
  (for _array_element_2 _outrownames
    (if (not (Utilities|Array|ContainsItem (LocalVariables|GetVisited) _array_element_2))
      (Development|PrintString (Utilities|String|Append "[Dialogue] ATTENTION : noeud inaccessible depuis les points d'entree : " (Utilities|String|ToString(Name) _array_element_2)) true true "(R=1.0,G=0.8,B=0.1,A=1.0)" 15.0))))

(fn LoadFlags
  (if (Variables|Sauvegarde|GetbPersistFlags)
    (bind _returnvalue (SaveGame|DoesSaveGameExist (Variables|Sauvegarde|GetSaveSlotName)))
    (if _returnvalue
      (bind _returnvalue_2 (SaveGame|LoadGamefromSlot (Variables|Sauvegarde|GetSaveSlotName)))
      (bind _asbp_dialogue_save (Utilities|Casting|CastToBP_DialogueSave _returnvalue_2))
      (Variables|Default|SetPlayerFlags (Variables|/Game/Blueprints/ClementTest/Dialogue/BP_DialogueSave.BP_DialogueSave_C|GetSavedFlags _asbp_dialogue_save))
      (Default|CallOnFlagsChanged))))

(fn SaveFlags
  (if (Variables|Sauvegarde|GetbPersistFlags)
    (bind _returnvalue (SaveGame|CreateSaveGameObject "/Game/Blueprints/ClementTest/Dialogue/BP_DialogueSave.BP_DialogueSave_C"))
    (Variables|/Game/Blueprints/ClementTest/Dialogue/BP_DialogueSave.BP_DialogueSave_C|SetSavedFlags _returnvalue (Variables|Default|GetPlayerFlags))
    (SaveGame|SaveGametoSlot _returnvalue (Variables|Sauvegarde|GetSaveSlotName))))

(fn ResetFlags
  (Variables|Default|SetPlayerFlags (GameplayTags|MakeLiteralGameplayTagContainer "(GameplayTags=)"))
  (SaveGame|DeleteGameinSlot (Variables|Sauvegarde|GetSaveSlotName))
  (Default|CallOnFlagsChanged)
  (Development|PrintString "[Dialogue] Tags du joueur remis a zero, sauvegarde effacee." true true "(R=0.000000,G=0.660000,B=1.000000,A=1.000000)" 5.0))