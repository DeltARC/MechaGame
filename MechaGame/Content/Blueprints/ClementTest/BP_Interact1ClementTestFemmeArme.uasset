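; Clickable test NPC actor for the FemmeArme quest dialogue, starting its DialogueNPC interaction when clicked.
; At BeginPlay it binds to the dialogue manager's OnChoiceSelected event to inspect the player's choices.
; When the last choice grants the Quete.FemmeArme.Acceptee tag, it sets Saidyes and plays the quest-button animation on the presenter's WBP_DialogueChoixFemmeArme widget.
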(event Custom|HandleChoiceSelected
  (bind _dialoguemanager (Default|GetManager (Variables|Default|GetDialogueNPC)))
  (if (GameplayTags|HasTag (.TagsToGrant (Utilities|Struct|BreakS_DialogueChoice (Variables|/Game/Blueprints/ClementTest/Dialogue/BP_DialogueManager.BP_DialogueManager_C|GetLastChoice _dialoguemanager))) (GameplayTags|MakeLiteralGameplayTag "(TagName=\"Quete.FemmeArme.Acceptee\")") true)
    (Variables|Default|SetSaidyes true)
    (bind _aswbp_dialogue_choix_femme_arme (Utilities|Casting|CastToWBP_DialogueChoixFemmeArme (Variables|/Game/Blueprints/ClementTest/Dialogue/BPC_DialoguePresenter.BPC_DialoguePresenter_C|GetWidget (Variables|/Game/Blueprints/ClementTest/Dialogue/BP_DialogueManager.BP_DialogueManager_C|GetDialoguePresenter _dialoguemanager))))
    (UserInterface|Animation|PlayAnimation _aswbp_dialogue_choix_femme_arme (Variables|/Game/Widgets/ClementTest/DialogueChoix/WBP_DialogueChoixFemmeArme.WBP_DialogueChoixFemmeArme_C|GetAnimationBoutonsQuetes _aswbp_dialogue_choix_femme_arme) 0.0 1 "Forward" 1.0 false)))

(event EventBeginPlay
  (bind _dialoguemanager (Default|GetManager (Variables|Default|GetDialogueNPC)))
  (EventDispatchers|BindEventtoOnChoiceSelected _dialoguemanager (EventDispatchers|CreateEvent :!event Custom|HandleChoiceSelected)))

(event Collision|EventActorBeginOverlap
  (params (OtherActor :type Actor%20Object%20Reference)))

(event EventTick
  (params (DeltaSeconds :type Float%20%28single-precision%29)))

(event MouseInput|EventActorOnClicked
  (params (ButtonPressed :type Key%20Structure :default "None"))
  (Default|Interact (Variables|Default|GetDialogueNPC)))

(fn ConstructionScript)