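; Quest log component for BP_DialogueManager that opens and closes a WBP_Quest screen, switching cursor and input and blocking player movement and look.
; It lists active and completed quests by checking their gameplay tags against the manager's PlayerFlags, with a completion counter, in five fixed button slots.
; Hovering or clicking a button finds its index by polling hover or focus, then fills the detail panel and highlights the selection.
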(event Custom|Open
  (bind _returnvalue (Game|GetPlayerController 0))
  (if (and (not (Variables|Default|GetbIsOpen)) (not (Variables|/Game/Blueprints/ClementTest/Dialogue/BP_DialogueManager.BP_DialogueManager_C|GetbIsActive (Variables|Default|GetManager))))
    (Variables|Default|SetbIsOpen true)
    (CallFunction|CreateLogWidget)
    (UserInterface|Viewport|AddtoViewport (Variables|Default|GetWidget) 10)
    (for _array_element (Variables|Default|GetQuestButtons)
      (EventDispatchers|BindEventtoOnClicked _array_element (EventDispatchers|CreateEvent :!event Custom|HandleQuestClicked))
      (EventDispatchers|BindEventtoOnHovered _array_element (EventDispatchers|CreateEvent :!event Custom|HandleQuestHovered)))
    (EventDispatchers|BindEventtoOnClicked (Variables|Default|GetCloseButton) (EventDispatchers|CreateEvent :!event Custom|HandleCloseClicked))
    (Variables|Default|SetbPreviousShowCursor (Variables|/Script/Engine.PlayerController|GetbShowMouseCursor _returnvalue))
    (Variables|/Script/Engine.PlayerController|SetbShowMouseCursor _returnvalue true)
    (Input|SetInputModeGameandUI _returnvalue 0 "DoNotLock" true false)
    (Input|SetIgnoreMoveInput _returnvalue true)
    (Input|SetIgnoreLookInput _returnvalue true)
    (CallFunction|RefreshList)))

(event Custom|Close
  (bind _returnvalue (Game|GetPlayerController 0))
  (if (Variables|Default|GetbIsOpen)
    (Variables|Default|SetbIsOpen false)
    (Widget|RemovefromParent (Variables|Default|GetWidget))
    (Variables|/Script/Engine.PlayerController|SetbShowMouseCursor _returnvalue (Variables|Default|GetbPreviousShowCursor))
    (Input|SetInputModeGameOnly _returnvalue false)
    (Input|SetIgnoreMoveInput _returnvalue false)
    (Input|SetIgnoreLookInput _returnvalue false)))

(event Custom|Toggle
  (if (Variables|Default|GetbIsOpen)
    (CallFunction|Close)
    (else
      (CallFunction|Open))))

(event Custom|HandleQuestHovered
  (bind _index (CallFunction|GetHoveredIndex))
  (if (>= _index (Class|KismetSystemLibrary|MakeLiteralInteger))
    (CallFunction|SelectQuest _index)))

(event Custom|HandleQuestClicked
  (bind _index (CallFunction|GetFocusedIndex))
  (if (>= _index (Class|KismetSystemLibrary|MakeLiteralInteger))
    (CallFunction|SelectQuest _index)
    (else
      (bind _index_2 (CallFunction|GetHoveredIndex))
      (if (>= _index_2 (Class|KismetSystemLibrary|MakeLiteralInteger))
        (CallFunction|SelectQuest _index_2)))))

(event Custom|HandleCloseClicked
  (CallFunction|Close))

(event EventBeginPlay
  (bind _asbp_dialogue_manager (Utilities|Casting|CastToBP_DialogueManager (Components|GetOwner))
    (:then
      (Variables|Default|SetManager _asbp_dialogue_manager))
    (:CastFailed
      (Development|PrintString "[Quetes] ERREUR : BPC_QuestLog doit etre un composant de BP_DialogueManager." true true "(R=1.0,G=0.2,B=0.2,A=1.0)" 15.0))))

(event EventTick
  (params (DeltaSeconds :type Float%20%28single-precision%29)))

(fn CreateLogWidget
  (Utilities|Array|Clear (Variables|Default|GetQuestButtons))
  (Utilities|Array|Clear (Variables|Default|GetQuestTitles))
  (Utilities|Array|Clear (Variables|Default|GetQuestLocations))
  (bind _returnvalue (UserInterface|CreateWidget "/Game/Widgets/ClementTest/Quetes/WBP_Quest.WBP_Quest_C" (Game|GetPlayerController 0)))
  (Variables|Default|SetWidget _returnvalue)
  (Utilities|Array|Add (Variables|Default|GetQuestButtons) (Variables|/Game/Widgets/ClementTest/Quetes/WBP_Quest.WBP_Quest_C|GetQuestButton1 _returnvalue))
  (Utilities|Array|Add (Variables|Default|GetQuestButtons) (Variables|/Game/Widgets/ClementTest/Quetes/WBP_Quest.WBP_Quest_C|GetQuestButton2 _returnvalue))
  (Utilities|Array|Add (Variables|Default|GetQuestButtons) (Variables|/Game/Widgets/ClementTest/Quetes/WBP_Quest.WBP_Quest_C|GetQuestButton3 _returnvalue))
  (Utilities|Array|Add (Variables|Default|GetQuestButtons) (Variables|/Game/Widgets/ClementTest/Quetes/WBP_Quest.WBP_Quest_C|GetQuestButton4 _returnvalue))
  (Utilities|Array|Add (Variables|Default|GetQuestButtons) (Variables|/Game/Widgets/ClementTest/Quetes/WBP_Quest.WBP_Quest_C|GetQuestButton5 _returnvalue))
  (Utilities|Array|Add (Variables|Default|GetQuestTitles) (Variables|/Game/Widgets/ClementTest/Quetes/WBP_Quest.WBP_Quest_C|GetQuestTitle1 _returnvalue))
  (Utilities|Array|Add (Variables|Default|GetQuestTitles) (Variables|/Game/Widgets/ClementTest/Quetes/WBP_Quest.WBP_Quest_C|GetQuestTitle2 _returnvalue))
  (Utilities|Array|Add (Variables|Default|GetQuestTitles) (Variables|/Game/Widgets/ClementTest/Quetes/WBP_Quest.WBP_Quest_C|GetQuestTitle3 _returnvalue))
  (Utilities|Array|Add (Variables|Default|GetQuestTitles) (Variables|/Game/Widgets/ClementTest/Quetes/WBP_Quest.WBP_Quest_C|GetQuestTitle4 _returnvalue))
  (Utilities|Array|Add (Variables|Default|GetQuestTitles) (Variables|/Game/Widgets/ClementTest/Quetes/WBP_Quest.WBP_Quest_C|GetQuestTitle5 _returnvalue))
  (Utilities|Array|Add (Variables|Default|GetQuestLocations) (Variables|/Game/Widgets/ClementTest/Quetes/WBP_Quest.WBP_Quest_C|GetQuestLocation1 _returnvalue))
  (Utilities|Array|Add (Variables|Default|GetQuestLocations) (Variables|/Game/Widgets/ClementTest/Quetes/WBP_Quest.WBP_Quest_C|GetQuestLocation2 _returnvalue))
  (Utilities|Array|Add (Variables|Default|GetQuestLocations) (Variables|/Game/Widgets/ClementTest/Quetes/WBP_Quest.WBP_Quest_C|GetQuestLocation3 _returnvalue))
  (Utilities|Array|Add (Variables|Default|GetQuestLocations) (Variables|/Game/Widgets/ClementTest/Quetes/WBP_Quest.WBP_Quest_C|GetQuestLocation4 _returnvalue))
  (Utilities|Array|Add (Variables|Default|GetQuestLocations) (Variables|/Game/Widgets/ClementTest/Quetes/WBP_Quest.WBP_Quest_C|GetQuestLocation5 _returnvalue))
  (Variables|Default|SetDetailTitle (Variables|/Game/Widgets/ClementTest/Quetes/WBP_Quest.WBP_Quest_C|GetDetailTitle _returnvalue))
  (Variables|Default|SetDetailGiver (Variables|/Game/Widgets/ClementTest/Quetes/WBP_Quest.WBP_Quest_C|GetDetailGiver _returnvalue))
  (Variables|Default|SetDetailLocation (Variables|/Game/Widgets/ClementTest/Quetes/WBP_Quest.WBP_Quest_C|GetDetailLocation _returnvalue))
  (Variables|Default|SetDetailDescription (Variables|/Game/Widgets/ClementTest/Quetes/WBP_Quest.WBP_Quest_C|GetDetailDescription _returnvalue))
  (Variables|Default|SetDetailCounter (Variables|/Game/Widgets/ClementTest/Quetes/WBP_Quest.WBP_Quest_C|GetDetailCounter _returnvalue))
  (Variables|Default|SetEmptyText (Variables|/Game/Widgets/ClementTest/Quetes/WBP_Quest.WBP_Quest_C|GetEmptyText _returnvalue))
  (Variables|Default|SetCloseButton (Variables|/Game/Widgets/ClementTest/Quetes/WBP_Quest.WBP_Quest_C|GetCloseButton _returnvalue)))

(fn RefreshList
  (Utilities|Array|Clear (Variables|Default|GetVisibleQuests))
  (Variables|Default|SetCompletedCount 0)
  (for _array_element (Variables|Default|GetQuests)
    (if (GameplayTags|HasTag (Variables|/Game/Blueprints/ClementTest/Dialogue/BP_DialogueManager.BP_DialogueManager_C|GetPlayerFlags (Variables|Default|GetManager)) (Variables|/Game/Blueprints/ClementTest/Quetes/BP_QuestData.BP_QuestData_C|GetCompletedTag _array_element) true)
      (Variables|Default|SetCompletedCount (+ (Variables|Default|GetCompletedCount) (Class|KismetSystemLibrary|MakeLiteralInteger 1)))
      (Utilities|Array|Add (Variables|Default|GetVisibleQuests) _array_element)
      (elif (GameplayTags|HasTag (Variables|/Game/Blueprints/ClementTest/Dialogue/BP_DialogueManager.BP_DialogueManager_C|GetPlayerFlags (Variables|Default|GetManager)) (Variables|/Game/Blueprints/ClementTest/Quetes/BP_QuestData.BP_QuestData_C|GetActiveTag _array_element) true)
        (Utilities|Array|Add (Variables|Default|GetVisibleQuests) _array_element))))
  (for _index (range 0 (- (Utilities|Array|Length (Variables|Default|GetQuestButtons)) (Class|KismetSystemLibrary|MakeLiteralInteger 1)))
    (if (< _index (Utilities|Array|Length (Variables|Default|GetVisibleQuests)))
      (Rendering|Components|TextRender|SetText (Utilities|Array|Get(acopy) (Variables|Default|GetQuestTitles) _index) (Variables|/Game/Blueprints/ClementTest/Quetes/BP_QuestData.BP_QuestData_C|GetTitle (Utilities|Array|Get(acopy) (Variables|Default|GetVisibleQuests) _index)))
      (if (GameplayTags|HasTag (Variables|/Game/Blueprints/ClementTest/Dialogue/BP_DialogueManager.BP_DialogueManager_C|GetPlayerFlags (Variables|Default|GetManager)) (Variables|/Game/Blueprints/ClementTest/Quetes/BP_QuestData.BP_QuestData_C|GetCompletedTag (Utilities|Array|Get(acopy) (Variables|Default|GetVisibleQuests) _index)) true)
        (Rendering|Components|TextRender|SetText (Utilities|Array|Get(acopy) (Variables|Default|GetQuestLocations) _index) (Variables|Default|GetCompletedLabel))
        (else
          (Rendering|Components|TextRender|SetText (Utilities|Array|Get(acopy) (Variables|Default|GetQuestLocations) _index) (Variables|/Game/Blueprints/ClementTest/Quetes/BP_QuestData.BP_QuestData_C|GetLocation (Utilities|Array|Get(acopy) (Variables|Default|GetVisibleQuests) _index)))))
      (Widget|SetVisibility (Utilities|Array|Get(acopy) (Variables|Default|GetQuestButtons) _index) "Visible")
      (else
        (Widget|SetVisibility (Utilities|Array|Get(acopy) (Variables|Default|GetQuestButtons) _index) "Collapsed"))))
  (Rendering|Components|TextRender|SetText (Variables|Default|GetDetailCounter) (Utilities|Text|ToText(String) (Utilities|String|Append (Utilities|String|ToString(Text) (Variables|Default|GetCounterLabel)) (Utilities|String|Append (Utilities|String|ToString(Integer) (Variables|Default|GetCompletedCount)) (Utilities|String|Append "/" (Utilities|String|ToString(Integer) (Utilities|Array|Length (Variables|Default|GetQuests))))))))
  (if (Utilities|Array|IsNotEmpty (Variables|Default|GetVisibleQuests))
    (Widget|SetVisibility (Variables|Default|GetEmptyText) "Collapsed")
    (CallFunction|SelectQuest)
    (Widget|SetKeyboardFocus (Utilities|Array|Get(acopy) (Variables|Default|GetQuestButtons)))
    (else
      (Variables|Default|SetSelectedIndex -1)
      (Widget|SetVisibility (Variables|Default|GetEmptyText) "Visible")
      (Rendering|Components|TextRender|SetText (Variables|Default|GetDetailTitle) (Variables|Default|GetNoQuestLabel))
      (Rendering|Components|TextRender|SetText (Variables|Default|GetDetailGiver) (Class|KismetTextLibrary|GetEmptyText))
      (Rendering|Components|TextRender|SetText (Variables|Default|GetDetailLocation) (Class|KismetTextLibrary|GetEmptyText))
      (Rendering|Components|TextRender|SetText (Variables|Default|GetDetailDescription) (Class|KismetTextLibrary|GetEmptyText))
      (Widget|SetKeyboardFocus (Variables|Default|GetCloseButton)))))

(fn SelectQuest
  (params (Index :type Integer))
  (if (Utilities|Array|IsValidIndex (Variables|Default|GetVisibleQuests) Index)
    (Variables|Default|SetSelectedIndex Index)
    (Rendering|Components|TextRender|SetText (Variables|Default|GetDetailTitle) (Variables|/Game/Blueprints/ClementTest/Quetes/BP_QuestData.BP_QuestData_C|GetTitle (Utilities|Array|Get(acopy) (Variables|Default|GetVisibleQuests) Index)))
    (Rendering|Components|TextRender|SetText (Variables|Default|GetDetailLocation) (Variables|/Game/Blueprints/ClementTest/Quetes/BP_QuestData.BP_QuestData_C|GetLocation (Utilities|Array|Get(acopy) (Variables|Default|GetVisibleQuests) Index)))
    (Rendering|Components|TextRender|SetText (Variables|Default|GetDetailDescription) (Variables|/Game/Blueprints/ClementTest/Quetes/BP_QuestData.BP_QuestData_C|GetDescription (Utilities|Array|Get(acopy) (Variables|Default|GetVisibleQuests) Index)))
    (for _index (range 0 (- (Utilities|Array|Length (Variables|Default|GetQuestButtons)) (Class|KismetSystemLibrary|MakeLiteralInteger 1)))
      (if (== _index Index)
        (Variables|/Script/UMG.Button|SetBackgroundColor (Utilities|Array|Get(acopy) (Variables|Default|GetQuestButtons) _index) (Variables|Default|GetSelectedColor))
        (else
          (Variables|/Script/UMG.Button|SetBackgroundColor (Utilities|Array|Get(acopy) (Variables|Default|GetQuestButtons) _index) (Variables|Default|GetNormalColor)))))
    (Utilities|IsValid (Variables|/Game/Blueprints/ClementTest/Quetes/BP_QuestData.BP_QuestData_C|GetGiver (Utilities|Array|Get(acopy) (Variables|Default|GetVisibleQuests) Index))
      (:Is%20Valid
        (Rendering|Components|TextRender|SetText (Variables|Default|GetDetailGiver) (Utilities|Text|ToText(String) (Utilities|String|Append (Utilities|String|ToString(Text) (Variables|Default|GetGiverPrefix)) (Utilities|String|ToString(Text) (Variables|/Game/Blueprints/ClementTest/Dialogue/BP_DialogueSpeakerData.BP_DialogueSpeakerData_C|GetDisplayName (Variables|/Game/Blueprints/ClementTest/Quetes/BP_QuestData.BP_QuestData_C|GetGiver (Utilities|Array|Get(acopy) (Variables|Default|GetVisibleQuests) Index))))))))
      (:Is%20Not%20Valid
        (Rendering|Components|TextRender|SetText (Variables|Default|GetDetailGiver) (Class|KismetTextLibrary|GetEmptyText))))))

(fn GetHoveredIndex
  (for _index (range 0 (- (Utilities|Array|Length (Variables|Default|GetQuestButtons)) (Class|KismetSystemLibrary|MakeLiteralInteger 1)))
    (if (Widget|IsHovered (Utilities|Array|Get(acopy) (Variables|Default|GetQuestButtons) _index))
      (return _index)))
  (return -1))

(fn GetFocusedIndex
  (for _index (range 0 (- (Utilities|Array|Length (Variables|Default|GetQuestButtons)) (Class|KismetSystemLibrary|MakeLiteralInteger 1)))
    (if (Class|Widget|HasKeyboardFocus (Utilities|Array|Get(acopy) (Variables|Default|GetQuestButtons) _index))
      (return _index)))
  (return -1))